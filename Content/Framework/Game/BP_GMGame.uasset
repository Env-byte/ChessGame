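; BP_GMGame is the game-side Blueprint that spawns and possesses a player pawn at the spawn point for that player's team.
; The SpawnPlayerCamera event passes player info to SpawnPlayer, then prints a debug message with the team.
; SpawnPlayer looks up the team in the PlayerSpawns map, always spawns BP_PlayerPawn there owned by the player's controller, and has it possessed, or prints an error if the team is missing.
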(event `self.BP_SpawnPlayerCamera`
  (params (PlayerInfo :type "PlayerInfo Structure (by ref)"))
  (`self.SpawnPlayer` PlayerInfo)
  (`KismetSystemLibrary.PrintText` (`|FormatText` "Spawned Actor Team {Team}" (`|GetEnumeratorNameAsString` (`.Team` (break `PlayerInfo` PlayerInfo)))) true true (struct :`G` 0.66 :`B` 1.0 :`A` 1.0) 10.0))

(fn `SpawnPlayer`
  (params (PlayerInfo :type "PlayerInfo Structure (by ref)"))
  (locals (ThisPlayerInfo :type "PlayerInfo Structure"))
  (bind ((`PlayerController` _playercontroller)) (break `PlayerInfo` (`local.ThisPlayerInfo`)))
  (bind _output_get (set `local.ThisPlayerInfo` PlayerInfo))
  (bind (_value _returnvalue) (`BlueprintMapLibrary.Map_Find` (`self.PlayerSpawns`) (`.Team` (break `PlayerInfo` _output_get))))
  (if _returnvalue
    (bind _returnvalue_2 (`|SpawnActorFromClass` "/Game/Framework/Game/BP_PlayerPawn.BP_PlayerPawn_C" (`self.GetTransform` _value) "AlwaysSpawn" "OverrideRootScale" _playercontroller null))
    (`Controller.Possess` _playercontroller _returnvalue_2)
    (else
      (`KismetSystemLibrary.PrintText` (`|FormatText` "Team Not Found {Team}" (`KismetStringLibrary.Conv_ByteToString` (`.Team` (break `PlayerInfo` (`local.ThisPlayerInfo`)))))))))

(fn `UserConstructionScript`)