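; BP_Tile is a single board tile with a mesh and a highlight decal, sized and coloured at BeginPlay.
; Mesh and decal scale from the TileController's width setting, with the decal at half scale and raised just above the mesh.
; Tiles whose TileInfo colour is not Black have their material tinted white.
; The indigo decal starts hidden, and AddHighlight and RemoveHighlight events toggle its visibility.
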(event `self.ReceiveBeginPlay`
  (bind (_returnvalue_x _returnvalue_y _returnvalue_z) (`KismetMathLibrary.BreakVector` (`SceneComponent.K2_GetComponentLocation` (`self.TileMesh`))))
  (bind _returnvalue (/ (`.Width` (break `TileControllerSettings` (`TileController.TileControllerSettings` (`self.TileController`)))) 100.0))
  (bind _returnvalue_2 (/ _returnvalue 2.0))
  (`|ExecutionSequence`
    (:`then_0`
      (`MeshComponent.SetVectorParameterValueOnMaterials` (`self.Decal`) "Colour" (75.0 0.0 130.0))
      (`self.BP_RemoveHighlight`))
    (:`then_1`
      (`SceneComponent.SetWorldScale3D` (`self.TileMesh`) (`KismetMathLibrary.MakeVector` _returnvalue _returnvalue))
      (`SceneComponent.SetWorldScale3D` (`self.Decal`) (`KismetMathLibrary.MakeVector` _returnvalue_2 _returnvalue_2))
      (`SceneComponent.K2_SetWorldLocation` (`self.Decal`) (`KismetMathLibrary.MakeVector` _returnvalue_x _returnvalue_y (+ _returnvalue_z 10.0)) false false)
      (if (not (`|EnumEquality` (`.TileColour` (break `TileInfo` (`self.TileInfo`))) "Black"))
        (`MeshComponent.SetVectorParameterValueOnMaterials` (`self.TileMesh`) "Colour" (255.0 255.0 255.0))))))

(event `self.BP_AddHighlight`
  (`SceneComponent.SetVisibility` (`self.Decal`) true false))

(event `self.BP_RemoveHighlight`
  (`SceneComponent.SetVisibility` (`self.Decal`) false false))

(fn `UserConstructionScript`)